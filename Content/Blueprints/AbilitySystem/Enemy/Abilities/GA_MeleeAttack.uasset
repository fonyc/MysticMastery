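; Enemy melee attack ability that warps toward the combat target and damages hostile live players.
; On activation it updates the facing warp target and plays a random tagged attack montage from the avatar.
; The montage's gameplay event triggers a small sphere query at the tagged combat socket, damaging non-friendly players and triggering their hit effects.
; A successful hit executes one MeleeImpact gameplay cue; the ability ends when the montage completes, interrupts or cancels.
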(event Ability|EventActivateAbility
  (bind _returnvalue (Ability|GetAvatarActorfromActorInfo))
  (bind _returnvalue_2 (Ability|GetAvatarActorfromActorInfo))
  (Variables|Default|SetbHitCausedDamage false)
  ;[1 1 1] Motion Warping
  (bind _returnvalue_3 (Class|EnemyInterface|GetCombatTarget(Message) _returnvalue))
  (bind _ascombat_interface (Utilities|Casting|CastToCombatInterface _returnvalue))
  (Class|CombatInterface|UpdateFacingWarpTarget _ascombat_interface (Transformation|GetActorLocation _returnvalue_3))
  ;[1 1 1] Retrieve the Tagged Montaged Variable (Includes animations, GameplayTag associated and the impact sound)
  (bind _returnvalue_4 (Class|CombatInterface|GetAttackMontages(Message) _returnvalue))
  (bind _output_get (Variables|Default|SetTaggedMontage (.OutItem (Utilities|Array|Random _returnvalue_4))))
  (|PlayMontageandWaitProxy "None" (.Montage (Utilities|Struct|BreakTaggedMontage _output_get)) 1.0 "None" true 1.0 0.0 false
    (:then
      (Ability|Tasks|WaitGameplayEvent (.MontageTag (Utilities|Struct|BreakTaggedMontage _output_get)) 0
        (:EventReceived
          (bind _returnvalue_5 (Class|CombatInterface|GetCombatSocketLocation(Message) _returnvalue_2 (.SocketTag (Utilities|Struct|BreakTaggedMontage _output_get))))
          (bind _output_get_2 (Variables|Default|SetCombatSocketLocation _returnvalue_5))
          (bind _outoverlappingactors (Class|MMAbilitySystemBlueprintLibrary|GetLivePlayersWithinRadius _returnvalue_2 (Utilities|Array|MakeArray _returnvalue_2) 6e+01 _output_get_2))
          (for _array_element _outoverlappingactors
            (if (not (Class|MMAbilitySystemBlueprintLibrary|IsFriendlyActor _array_element (Ability|GetAvatarActorfromActorInfo)))
              (Class|MMDamageGameplayAbility|CauseDamage _array_element)
              (Variables|Default|SetbHitCausedDamage true)
              (Class|CombatInterface|GetHitEffect(Message) _array_element)))
          ;[1 1 1] If the hit caused damage, at the end of the loop, play a sound / sfx via CUES
          (if (Variables|Default|GetbHitCausedDamage)
            (bind _returnvalue_6 (Class|EnemyInterface|GetCombatTarget(Message) (Ability|GetAvatarActorfromActorInfo)))
            (Class|GameplayAbility|ExecuteGameplayCuewithParams "(TagName=\"GameplayCue.MeleeImpact\")" (Ability|GameplayCue|MakeGameplayCueParameters :AggregatedSourceTags (GameplayTags|MakeGameplayTagContainerfromTag (.MontageTag (Utilities|Struct|BreakTaggedMontage (Variables|Default|GetTaggedMontage)))) :Location (Variables|Default|GetCombatSocketLocation) :EffectCauser (Ability|GetAvatarActorfromActorInfo) :SourceObject _returnvalue_6))))))
    (:OnCompleted
      (Ability|EndAbility :!label _label))
    (:OnInterrupted
      (goto _label))
    (:OnCancelled
      (goto _label))))