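; Enemy gameplay ability that summons random minions, using the Goblin Shaman summon montage.
; On activation it shuffles the spawn locations, places summon-circle VFX at each and plays the montage.
; A montage gameplay event starts a staggered, delay-driven loop that spawns AI-possessed minions facing away from the summoner.
; The summoner's minion count rises per spawn and falls through each minion's OnDestroyed binding.
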(event Custom|OnDestroyed_Event
  (params (DestroyedActor :type Actor%20Object%20Reference))
  ;[1 1 1] Bind On Destroy Event to Decrement the number of minions of the summoner
  (Class|CombatInterface|IncrementMinionCount(Message) (Ability|GetAvatarActorfromActorInfo) -1))

(event Ability|EventActivateAbility
  (Variables|Default|SetSpawnLocationIndex 0)
  (bind _returnvalue (Class|MMSummonAbility|GetSpawnLocations))
  (bind _output_get (Variables|Default|SetSpawnLocations _returnvalue))
  (Utilities|Array|Shuffle _output_get)
  ;[1 1 1] Spawn VFX in the places that the minions will be spawned
  (for _array_element _output_get
    (Niagara|SpawnSystematLocation "/Game/Assets/sA_StylizedWizardSet/Fx/NS_SummonCircle.NS_SummonCircle" (+ _array_element "0.000000,0.000000,15.000000")))
  (|PlayMontageandWaitProxy "None" "/Game/Animations/Synty/Shaman/AM_GoblinShaman_Summon.AM_GoblinShaman_Summon" 1.0 "None" true 1.0 0.0 false
    (:then
      (Ability|Tasks|WaitGameplayEvent "(TagName=\"Montage.Attack.1\")" 0
        (:EventReceived
          (if (< (Variables|Default|GetSpawnLocationIndex) (Utilities|Array|Length (Variables|Default|GetSpawnLocations))) :!label _label
            (bind _returnvalue_2 (Game|SpawnActorfromClass (Class|MMSummonAbility|GetRandomMinionClass) (Math|Transform|MakeTransform (+ (Utilities|Array|Get(acopy) (Variables|Default|GetSpawnLocations) (Variables|Default|GetSpawnLocationIndex)) "0.000000,0.000000,70.000000") (Math|Rotator|FindLookatRotation (Transformation|GetActorLocation (Ability|GetAvatarActorfromActorInfo)) (+ (Utilities|Array|Get(acopy) (Variables|Default|GetSpawnLocations) (Variables|Default|GetSpawnLocationIndex)) "0.000000,0.000000,70.000000")) "1.000000,1.000000,1.000000") "Undefined" "MultiplyWithRoot" 0 0))
            (Utilities|IsValid _returnvalue_2
              (:Is%20Valid
                (Game|AssignOnDestroyed _returnvalue_2 (delegate Custom|OnDestroyed_Event))
                (Pawn|SpawnDefaultController _returnvalue_2)
                (Class|CombatInterface|IncrementMinionCount(Message) (Ability|GetAvatarActorfromActorInfo) 1)
                (Math|Integer|IncrementInt (Variables|Default|GetSpawnLocationIndex)
                  (:%20%20
                    (Utilities|FlowControl|Delay 0.1)
                    (goto _label))))
              (:Is%20Not%20Valid
                (Math|Integer|IncrementInt (Variables|Default|GetSpawnLocationIndex)
                  (:%20%20
                    (goto _label)))))))))
    (:OnCompleted
      (Ability|EndAbility :!label _label_2))
    (:OnInterrupted
      (goto _label_2))
    (:OnCancelled
      (goto _label_2))))

(event Ability|EventOnEndAbility
  (params (bWasCancelled :type Boolean)))