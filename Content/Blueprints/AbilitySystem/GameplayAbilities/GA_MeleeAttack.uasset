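; GA_MeleeAttack is a gameplay ability for a melee attack, using the goblin spear attack montage.
; On activation it sets the avatar's facing warp target to its combat target's location through CombatInterface, then plays the montage.
; When the Event.Montage.Attack.Melee event arrives, it only draws a debug sphere at the combat socket, with no damage applied.
; The ability ends when the montage completes, is interrupted or is cancelled.
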(event Ability|EventActivateAbility
  (bind _returnvalue (Ability|GetAvatarActorfromActorInfo))
  (bind _returnvalue_2 (Class|EnemyInterface|GetCombatTarget(Message) _returnvalue))
  (bind _ascombat_interface (Utilities|Casting|CastToCombatInterface _returnvalue))
  (Class|CombatInterface|UpdateFacingWarpTarget _ascombat_interface (Transformation|GetActorLocation _returnvalue_2))
  (|PlayMontageandWaitProxy "None" "/Game/Animations/Synty/Animations/Goblin_Spear/AM_GoblinSpear_Attack.AM_GoblinSpear_Attack" 1.0 "None" true 1.0 0.0 false
    (:then
      (Ability|Tasks|WaitGameplayEvent "(TagName=\"Event.Montage.Attack.Melee\")" 0
        (:EventReceived
          (bind _returnvalue_3 (Class|CombatInterface|GetCombatSocketLocation(Message) (Ability|GetAvatarActorfromActorInfo)))
          (Rendering|Debug|DrawDebugSphere _returnvalue_3 45.0 12 "(R=1.000000,G=0.057804,B=0.000000,A=1.000000)" 3.0 2.0))))
    (:OnCompleted
      (Ability|EndAbility :!label _label))
    (:OnInterrupted
      (goto _label))
    (:OnCancelled
      (goto _label))))

(event Ability|EventOnEndAbility
  (params (bWasCancelled :type Boolean)))