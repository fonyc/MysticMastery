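; Mage Fire Bolt gameplay ability that fires a projectile at the point under the mouse cursor.
; On valid target data it stores the hit location, updates the avatar's facing warp target through CombatInterface and plays the cast montage.
; A montage gameplay event triggers SpawnProjectile from the weapon socket tag.
; A temporary delay before EndAbility keeps the client from ending the ability too soon.
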(event Ability|EventActivateAbility
  (Ability|CommitAbility)
  (bind _datahandle (|TargetDataUnderMouse)
    (:ValidData
      (Variables|Default|SetProjectileTarget (.Location (Collision|BreakHitResult (Ability|TargetData|GetHitResultfromTargetData _datahandle))))
      ;[1 1 1] Set the location for the warping animation
      (bind _ascombat_interface (Utilities|Casting|CastToCombatInterface (Ability|GetAvatarActorfromActorInfo))
        (:then
          (Class|CombatInterface|UpdateFacingWarpTarget _ascombat_interface (Variables|Default|GetProjectileTarget)))
        (:CastFailed
          _))
      (|PlayMontageandWaitProxy "None" "/Game/Animations/Synty/Mage/AM_Mage_FireBolt.AM_Mage_FireBolt" 1.0 "None" true 1.0 0.0 false
        (:then
          (Ability|Tasks|WaitGameplayEvent "(TagName=\"Event.Montage.CastFireBolt\")" 0
            (:EventReceived
              (Class|MMProjectileSpell|SpawnProjectile (Variables|Default|GetProjectileTarget) (GameplayTags|MakeLiteralGameplayTag "(TagName=\"CombatSocket.Weapon\")"))
              ;[1 1 1] Temporary delay. If its not placed here, the client ends its ability too soon and cannot perform GA
              (Utilities|FlowControl|Delay 0.5)
              (Ability|EndAbility))))))))

(event Ability|EventOnEndAbility
  (params (bWasCancelled :type Boolean)))