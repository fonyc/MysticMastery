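; Channeled Mage lightning ability that fires an electric beam at the target under the mouse while input is held.
; It warps facing toward the cursor and plays a cast montage, whose event locks movement and starts the shock loop.
; The beam is a ShockLoop gameplay cue placed on the hit combat actor, otherwise on the caster.
; Release restores cursor and movement, removes the cue, and debug-draws additional targets and radius.
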(event Ability|EventActivateAbility
  (CallFunction|CheckImplementsCombatInterface)
  ;[1 1 1] Set up neccesary data from mouse click
  (bind _datahandle (|TargetDataUnderMouse)
    (:ValidData
      (Class|MMBeamSpell|StoreMouseDataInfo (Ability|TargetData|GetHitResultfromTargetData _datahandle))
      (Class|MMBeamSpell|StoreOwnerPlayerControllerandCharacter)
      (Utilities|FlowControl|Sequence
        (:then_0
          (Variables|/Script/Engine.PlayerController|SetbShowMouseCursor (Variables|Default|GetOwnerPlayerController) false)
          (Class|CombatInterface|UpdateFacingWarpTarget(Message) (Ability|GetAvatarActorfromActorInfo) (Variables|Default|GetMouseLocation))
          (GameplayCue|ExecuteGameplayCue :GameplayCueTag "(TagName=\"GameplayCue.ShockBurst\")")
          (|PlayMontageandWaitProxy "None" (Variables|Default|GetMontage_Electrocute) 1.0 "None" true 1.0 0.0 false
            (:then
              (Ability|Tasks|WaitGameplayEvent "(TagName=\"Event.Montage.CastElectrocute\")" 0 true
                (:EventReceived
                  (CallFunction|InShockLoopActions)
                  (CallFunction|SpawnElectricBeam))))))
        (:then_1
          (Ability|Tasks|WaitInputRelease false
            (:OnRelease
              (CallFunction|BeforeEndAbilityActions)
              (Ability|EndAbility))))))))

(fn CheckImplementsCombatInterface
  (if (Utilities|DoesObjectImplementInterface (Ability|GetAvatarActorfromActorInfo) "/Script/MysticMastery.CombatInterface")
    _))

(fn SetCharacterMovement
  (params (bEnable :type Boolean))
  (if bEnable
    (Pawn|Components|CharacterMovement|SetMovementMode (Variables|/Script/Engine.Character|GetCharacterMovement (Variables|Default|GetOwnerCharacter)) "MOVE_Walking" 0)
    (else
      (Pawn|Components|CharacterMovement|DisableMovement (Variables|/Script/Engine.Character|GetCharacterMovement (Variables|Default|GetOwnerCharacter))))))

(fn BeforeEndAbilityActions
  (Variables|/Script/Engine.PlayerController|SetbShowMouseCursor (Variables|Default|GetOwnerPlayerController) true)
  (Class|CombatInterface|SetinShockLoop(Message) (Ability|GetAvatarActorfromActorInfo) false)
  (CallFunction|SetCharacterMovement true)
  (if (Variables|Default|GetbFirstTargetImplementsInterface)
    (GameplayCue|RemoveGameplayCueOnActor(Looping) (Variables|Default|GetMouseHitActor) "(TagName=\"GameplayCue.ShockLoop\")" (Variables|Default|GetFirstTargetCueParams))
    (else
      (GameplayCue|RemoveGameplayCue "(TagName=\"GameplayCue.ShockLoop\")")))
  (bind _outadditionaltargets (Class|MMBeamSpell|StoreAdditionalTargets))
  (for _array_element _outadditionaltargets
    (Rendering|Debug|DrawDebugSphere (Transformation|GetActorLocation _array_element) 5e+01 12 "(R=1.000000,G=0.099114,B=0.000000,A=1.000000)" 3e+01 2.0))
  (Rendering|Debug|DrawDebugSphere (Transformation|GetActorLocation (Variables|Default|GetMouseHitActor)) (Class|MMBeamSpell|GetRadiusfromCurveTable) 12 "(R=0.097973,G=0.090404,B=1.000000,A=1.000000)" 3e+01 2.0))

(fn InShockLoopActions
  (Class|CombatInterface|SetinShockLoop(Message) (Ability|GetAvatarActorfromActorInfo) true)
  (CallFunction|SetCharacterMovement false))

(fn SpawnElectricBeam
  (Class|MMBeamSpell|TraceFirstTarget (Variables|Default|GetMouseLocation))
  (bind _returnvalue (Class|CombatInterface|GetWeapon(Message) (Ability|GetAvatarActorfromActorInfo)))
  (Variables|Default|SetFirstTargetCueParams (Ability|GameplayCue|MakeGameplayCueParameters :Location (Variables|Default|GetMouseLocation) :SourceObject (Variables|Default|GetMouseHitActor) :TargetAttachComponent _returnvalue))
  ;[1 1 1] Check Mouse Hit Actor is an enemy (if its true: apply the cue to an enemy, else add it to the avatar actor)
  (bind _output_get (Variables|Default|SetbFirstTargetImplementsInterface (Utilities|DoesObjectImplementInterface (Variables|Default|GetMouseHitActor) "/Script/MysticMastery.CombatInterface")))
  (if _output_get
    (LocalVariables|SetCueTarget (Variables|Default|GetMouseHitActor))
    (else
      (LocalVariables|SetCueTarget (Ability|GetAvatarActorfromActorInfo))))
  (GameplayCue|AddGameplayCueOnActor(Looping) (LocalVariables|GetCueTarget) "(TagName=\"GameplayCue.ShockLoop\")" (Variables|Default|GetFirstTargetCueParams)))