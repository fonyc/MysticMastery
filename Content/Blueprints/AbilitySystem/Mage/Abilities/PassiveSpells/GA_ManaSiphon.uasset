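; GA_ManaSiphon is the Mage's passive Mana Siphon gameplay ability.
; On activation it applies the GE_ManaSiphon effect to its owner at the ability's level and stores the active effect handle.
; When the ability ends, it removes all stacks of that effect from the avatar's Ability System Component, with debug prints marking both events.
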(event Ability|EventActivateAbility
  (Development|PrintString "Mana Siphon Activated" true true "(R=0.000000,G=0.660000,B=1.000000,A=1.000000)" 5.0)
  (bind _returnvalue (Ability|ApplyGameplayEffectSpecToOwner (Ability|MakeOutgoingGameplayEffectSpec "/Game/Blueprints/AbilitySystem/Mage/Abilities/PassiveSpells/GE_ManaSiphon.GE_ManaSiphon_C" (Math|Conversions|ToFloat(Integer) (Ability|GetAbilityLevel)))))
  (Variables|Default|SetAbilitySpec _returnvalue))

(event Ability|EventOnEndAbility
  (params (bWasCancelled :type Boolean))
  (Development|PrintString "Mana SiphonProtection Ends" true true "(R=1.000000,G=0.145833,B=0.145833,A=1.000000)" 5.0)
  (GameplayEffects|RemoveActiveGameplayEffect (Ability|GetAbilitySystemComponent (Ability|GetAvatarActorfromActorInfo)) (Variables|Default|GetAbilitySpec) -1))