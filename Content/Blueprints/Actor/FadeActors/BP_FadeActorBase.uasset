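; Base actor for a static mesh that can fade out and back in.
; Construction caches original materials and creates dynamic instances from faded material variants.
; FadeOut swaps those instances onto the mesh and plays a timeline driving their Fade parameter, which Fadein reverses.
; When finished, a faded-out mesh stops casting shadows and ignores a custom trace channel, while a faded-in mesh regains its original materials, shadows and blocking.
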(event EventFadein
  (bind _fadevalue (Timeline|Fade%20Timeline Reverse)
    (:Update
      (for _array_element (Variables|Default|GetDynamicInstances)
        (Rendering|Material|SetScalarParameterValue _array_element "Fade" _fadevalue :!class /Script/Engine.MaterialInstanceDynamic)))
    (:Finished
      (CallFunction|FadeFinishedActions _fadevalue))))

(event EventFadeOut
  (CallFunction|SetMaterialstoDynamicInstances)
  (bind _fadevalue (Timeline|Fade%20Timeline Play)
    (:Update
      (for _array_element (Variables|Default|GetDynamicInstances)
        (Rendering|Material|SetScalarParameterValue _array_element "Fade" _fadevalue :!class /Script/Engine.MaterialInstanceDynamic)))
    (:Finished
      (CallFunction|FadeFinishedActions _fadevalue))))

(fn ConstructionScript
  (Utilities|Array|Clear (Variables|Default|GetDynamicInstances))
  (Variables|Default|SetStartingMaterials (Rendering|Material|GetMaterials (Variables|Default|GetStaticMesh)))
  (for _array_element (Variables|Default|GetFadedMaterialInstances)
    (bind _returnvalue (Rendering|Material|CreateDynamicMaterialInstance _array_element "None" "None" :!class /Script/Engine.KismetMaterialLibrary))
    (Utilities|Array|AddUnique (Variables|Default|GetDynamicInstances) _returnvalue)))

(fn SetMaterialstoDynamicInstances
  (for (_array_element _array_index) (Variables|Default|GetDynamicInstances)
    (Rendering|Material|SetMaterial (Variables|Default|GetStaticMesh) _array_index _array_element)))

(fn ResetMaterialstoStartingValues
  (for (_array_element _array_index) (Variables|Default|GetStartingMaterials)
    (Rendering|Material|SetMaterial (Variables|Default|GetStaticMesh) _array_index _array_element)))

(fn FadeFinishedActions
  (params (InputPin :type Float%20%28single-precision%29))
  ;[1 1 1] Fade In
  (if (>= InputPin 1.0)
    (CallFunction|ResetMaterialstoStartingValues)
    (Rendering|SetCastShadow (Variables|Default|GetStaticMesh) true)
    (Collision|SetCollisionResponsetoChannel (Variables|Default|GetStaticMesh) "ECC_GameTraceChannel2" "ECR_Block")
    (else
      ;[1 1 1] Fade Out
      (if (<= InputPin 0.2)
        (Rendering|SetCastShadow (Variables|Default|GetStaticMesh) false)
        (Collision|SetCollisionResponsetoChannel (Variables|Default|GetStaticMesh) "ECC_GameTraceChannel2" "ECR_Ignore")))))