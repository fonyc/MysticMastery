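; Candle actor that flickers its FireLight point light to imitate a live flame.
; On BeginPlay it stores the light's starting intensity, then loops: short random delay, play a flicker timeline, choose again when it finishes.
; Timeline values are multiplied by IntensityScaler and added to the starting intensity.
; Two timelines are wired for random selection, but RandomInteger(1) always returns 0, so only the first branch is selected.
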(event Custom|PlayTimeline_2
  (bind _pointlight_intensity_2 (Timeline|Timeline_2 PlayFromStart)
    (:Update
      (CallFunction|ChangeFlameIntensity _pointlight_intensity_2))
    (:Finished
      (CallFunction|ChooseTimelineRandomly))))

(event Custom|Choose%20Timeline%20Randomly
  (Utilities|FlowControl|Delay (Math|Random|RandomFloatinRange 0.1 0.2))
  (switch int (Math|Random|RandomInteger 1)
    (:0
      (CallFunction|PlayTimeline1))
    (:1
      (CallFunction|PlayTimeline2))))

(event Custom|Play%20Timeline_1
  (bind _pointlightntensity_1 (Timeline|Timeline_1 PlayFromStart)
    (:Update
      (CallFunction|ChangeFlameIntensity _pointlightntensity_1))
    (:Finished
      (CallFunction|ChooseTimelineRandomly))))

(event EventBeginPlay
  ;[1 1 1] Get Initial Light intensity from the point light (Candelas)
  (Variables|Default|SetStartingIntensity (Variables|/Script/Engine.LightComponentBase|GetIntensity (Variables|Default|GetFireLight)))
  (CallFunction|ChooseTimelineRandomly))

(fn ConstructionScript)

(fn ChangeFlameIntensity
  (params (A :type Float%20%28double-precision%29))
  (Rendering|Components|Light|SetIntensity (Variables|Default|GetFireLight) (+ (* A (Variables|Default|GetIntensityScaler)) (Variables|Default|GetStartingIntensity))))