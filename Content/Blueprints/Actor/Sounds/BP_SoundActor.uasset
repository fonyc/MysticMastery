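; BP_SoundActor is an actor that plays a sound at its own location when play begins.
; BeginPlay fires a one-shot PlaySoundAtLocation using its sound and attenuation settings variables at a low, fixed volume.
; A helper function reads falloff distance and cone sphere radius from attenuation settings, but the event graph logic that stores them never runs.
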(event EventBeginPlay
  (Audio|PlaySoundatLocation (Variables|Default|GetSoundBase) (Transformation|GetActorLocation) "0, 0, 0" 0.1 1.0 0.0 (Variables|Default|GetAttenuation%20Settings) 0 0 0))

(fn ConstructionScript)

(fn GetAttenuationandFallofffromAttenuationSettings
  (params (self2 :type Sound%20Attenuation%20Object%20Reference))
  (bind _attenuation (Variables|/Script/Engine.SoundAttenuation|GetAttenuation self2))
  (return (.falloffdistance _attenuation) (.conesphereradius _attenuation)))