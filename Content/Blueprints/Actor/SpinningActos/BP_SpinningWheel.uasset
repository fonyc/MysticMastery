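; Animated spinning wheel actor with a rotating mechanism and two sets of chains that travel vertically in opposite directions.
; Tick rolls the wheel, pitches the mechanism and moves the chains at wheel speed, with one flag setting the direction.
; Chains passing the UpMark or DownMark shift back by the distance between them, forming an endless loop.
; The construction script fills the chain sets, and BeginPlay starts the chain sound at the actor's location.
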(event EventBeginPlay
  ;[1 1 1] Init Chain Loop Sound
  (Audio|PlaySoundatLocation "/Game/Assets/Sounds/Lever/Chains.Chains" (Transformation|GetActorLocation) "0, 0, 0" 0.05 1.0 0.0 "/Game/Assets/Sounds/Abilities/FireBolt/att_InWorld.att_InWorld" 0 0 0))

(event EventTick
  (params (DeltaSeconds :type Float%20%28single-precision%29))
  (CallFunction|WheelRotation DeltaSeconds (Variables|SpinSettings|GetInvertWheelRotation))
  (CallFunction|MechanismRotation DeltaSeconds (not (Variables|SpinSettings|GetInvertWheelRotation)))
  (CallFunction|MoveChains DeltaSeconds (Variables|ChainSettings|GetChain%20Set%202) (Variables|SpinSettings|GetInvertWheelRotation))
  (CallFunction|MoveChains DeltaSeconds (Variables|ChainSettings|GetChain%20Set%201) (not (Variables|SpinSettings|GetInvertWheelRotation))))

(fn ConstructionScript
  (bind _chain_set_1 (Variables|ChainSettings|GetChain%20Set%201))
  (bind _chain_set_2 (Variables|ChainSettings|GetChain%20Set%202))
  (Utilities|Array|AddUnique _chain_set_1 (Variables|Default|GetUpChain_1))
  (Utilities|Array|AddUnique _chain_set_1 (Variables|Default|GetUpChain_2))
  (Utilities|Array|AddUnique _chain_set_1 (Variables|Default|GetUpChain_3))
  (Utilities|Array|AddUnique _chain_set_2 (Variables|Default|GetDownChain_1))
  (Utilities|Array|AddUnique _chain_set_2 (Variables|Default|GetDownChain_2))
  (Utilities|Array|AddUnique _chain_set_2 (Variables|Default|GetDownChain_3)))

(fn WheelRotation
  (params (DeltaRotation :type Float%20%28double-precision%29) (InverseRotation :type Boolean))
  (if InverseRotation
    (LocalVariables|SetSpinDirection -1.0)
    (else
      (LocalVariables|SetSpinDirection 1.0)))
  (Transformation|AddLocalRotation (Variables|Default|GetWheel) (Math|Rotator|MakeRotator (* DeltaRotation (LocalVariables|GetSpinDirection) (Variables|SpinSettings|GetWheelSpinSpeed)) 0.0 0.0) false false))

(fn MechanismRotation
  (params (Delta%20Rotation :type Float%20%28single-precision%29) (Inverse%20Rotation :type Boolean))
  (if Inverse%20Rotation
    (LocalVariables|SetSpinDirection 1.0)
    (else
      (LocalVariables|SetSpinDirection -1.0)))
  (Transformation|AddLocalRotation (Variables|Default|GetMechanism) (Math|Rotator|MakeRotator 0.0 (* Delta%20Rotation (LocalVariables|GetSpinDirection) (Variables|SpinSettings|GetMechanismSpinSpeed)) 0.0) false false))

(fn MoveChains
  (params (DeltaLocation_Z :type Float%20%28double-precision%29) (Up%20Chains :type Array%20of%20Scene%20Component%20Object%20References) (Reverse :type Boolean))
  (bind _output_get (LocalVariables|SetbIsReversed Reverse))
  (if _output_get
    (LocalVariables|SetDirectionModifier -1.0)
    (else
      (LocalVariables|SetDirectionModifier 1.0)))
  (if (LocalVariables|GetbIsReversed)
    (LocalVariables|SetSelectedMark (Variables|Default|GetDownMark))
    (else
      (LocalVariables|SetSelectedMark (Variables|Default|GetUpMark))))
  (for _array_element Up%20Chains
    (bind _output_get_2 (LocalVariables|SetSelected%20Chain _array_element))
    (Transformation|AddLocalOffset _output_get_2 (Math|Vector|MakeVector 0.0 0.0 (* DeltaLocation_Z (LocalVariables|GetDirectionModifier) (Variables|SpinSettings|GetWheelSpinSpeed))) false false)
    (if (LocalVariables|GetbIsReversed)
      (bind _returnvalue (CallFunction|IsChainLessorEqualThantheMark (LocalVariables|GetSelected%20Chain) (LocalVariables|GetSelectedMark)))
      (LocalVariables|SetbDidItReachPosition _returnvalue)
      (else
        (bind _returnvalue_2 (CallFunction|IsChainGraterorEqualThanMark (LocalVariables|GetSelected%20Chain) (LocalVariables|GetSelectedMark)))
        (LocalVariables|SetbDidItReachPosition _returnvalue_2)))
    (if (LocalVariables|GetbDidItReachPosition)
      (Transformation|AddLocalOffset (LocalVariables|GetSelected%20Chain) (Math|Vector|MakeVector 0.0 0.0 (* (- (.z (Transformation|GetWorldLocation (Variables|Default|GetUpMark))) (.z (Transformation|GetWorldLocation (Variables|Default|GetDownMark)))) (* (LocalVariables|GetDirectionModifier) -1.0))) false false))))

(fn IsChainGraterorEqualThanMark
  (params (SelectedChain :type Scene%20Component%20Object%20Reference) (SelectedMark :type Scene%20Component%20Object%20Reference))
  (return (>= (.z (Transformation|GetWorldLocation SelectedChain)) (.z (Transformation|GetWorldLocation SelectedMark)))))

(fn IsChainLessorEqualThantheMark
  (params (SelectedChain :type Scene%20Component%20Object%20Reference) (SelectedMark :type Scene%20Component%20Object%20Reference))
  (return (<= (.z (Transformation|GetWorldLocation SelectedChain)) (.z (Transformation|GetWorldLocation SelectedMark)))))